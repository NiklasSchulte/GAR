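; Elevator Blueprint (Fahrstuhl) that moves its Cube from a start position to an end position while an actor overlaps its Trigger.
; Any overlap by another actor plays the Fahrstuhl timeline, and ending an overlap reverses it from its current point.
; The timeline's Alpha interpolates between the AusgangsPosition and EndPosition world locations without sweep, at a PlayRate set on BeginPlay.
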(event OnComponentBeginOverlap(Trigger)
  (params (OverlappedComponent :type Primitive%20Component%20Object%20Reference) (OtherActor :type Actor%20Object%20Reference) (OtherComp :type Primitive%20Component%20Object%20Reference) (OtherBodyIndex :type Integer) (bFromSweep :type Boolean) (SweepResult :type Hit%20Result%20Structure%20%28by%20ref%29))
  (if (not (== OtherActor self))
    (bind _alpha (Timeline|Fahrstuhl Play)
      (:Update
        (Transformation|SetWorldLocation (Variables|Default|GetCube) (Math|Vector|Lerp(Vector) (Transformation|GetWorldLocation (Variables|Default|GetAusgangsPosition)) (Transformation|GetWorldLocation (Variables|Default|GetEndPosition)) _alpha) false false)))))

(event OnComponentEndOverlap(Trigger)
  (params (OverlappedComponent :type Primitive%20Component%20Object%20Reference) (OtherActor :type Actor%20Object%20Reference) (OtherComp :type Primitive%20Component%20Object%20Reference) (OtherBodyIndex :type Integer))
  (if (not (== OtherActor self))
    (bind _alpha (Timeline|Fahrstuhl Reverse)
      (:Update
        (Transformation|SetWorldLocation (Variables|Default|GetCube) (Math|Vector|Lerp(Vector) (Transformation|GetWorldLocation (Variables|Default|GetAusgangsPosition)) (Transformation|GetWorldLocation (Variables|Default|GetEndPosition)) _alpha) false false)))))

(event EventBeginPlay
  (Components|Timeline|SetPlayRate (Variables|Default|GetFahrstuhl) (Variables|Default|GetPlayRate)))

(fn ConstructionScript)