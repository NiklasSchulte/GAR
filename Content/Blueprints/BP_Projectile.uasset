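; BP_Projectile is a projectile Blueprint built on a ProjectileMovement component and a Sphere component.
; Its Construction Script copies the velocity, gravity scale and bounce variables onto the movement component, then applies the collision and physics-simulation settings to the sphere.
; The event graph holds only disabled default events, so the Blueprint adds no runtime hit or overlap logic.
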(event EventBeginPlay)

(event Collision|EventActorBeginOverlap
  (params (OtherActor :type Actor%20Object%20Reference)))

(event EventTick
  (params (DeltaSeconds :type Float%20%28single-precision%29)))

(fn ConstructionScript
  (bind _projectilemovement (Variables|Default|GetProjectileMovement))
  (Variables|/Script/Engine.MovementComponent|SetVelocity _projectilemovement (Variables|Default|GetVelocity))
  (Variables|/Script/Engine.ProjectileMovementComponent|SetProjectileGravityScale _projectilemovement (Variables|Default|GetProjectile%20Gravity%20Scale))
  (Variables|/Script/Engine.ProjectileMovementComponent|SetbShouldBounce _projectilemovement (Variables|Default|GetShould%20Bounce))
  (Collision|SetCollisionEnabled (Variables|Default|GetSphere) (Variables|Default|GetCollision))
  (Physics|SetSimulatePhysics (Variables|Default|GetSphere) (Variables|Default|GetSimulate)))