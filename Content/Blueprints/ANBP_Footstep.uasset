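; Animation notify that plays a surface-dependent footstep sound for the left or right foot.
; The Foot setting selects a foot socket on the mesh, and a Visibility line trace runs straight down from it, ignoring the owner.
; The hit physical material's surface type keys into the Sound map, and the result plays at the impact location.
; The trace leaves timed debug lines on screen.
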(fn ReceivedNotify
  (params (MeshComp :type Skeletal%20Mesh%20Component%20Object%20Reference) (Animation :type Anim%20Sequence%20Base%20Object%20Reference) (EventReference :type Anim%20Notify%20Event%20Reference%20Structure%20%28by%20ref%29))
  (Utilities|IsValid MeshComp
    (:Is%20Valid
      (switch Utilities|FlowControl|Switch|SwitchonFootside (Variables|Default|GetFoot)
        (:NewEnumerator0
          (LocalVariables|SetSocketName "foot_l_Socket"))
        (:NewEnumerator1
          (LocalVariables|SetSocketName "foot_r_Socket")))
      (bind _outhit (Collision|LineTraceByChannel (Transformation|GetSocketLocation MeshComp (LocalVariables|GetSocketName)) (- (Transformation|GetSocketLocation MeshComp (LocalVariables|GetSocketName)) "0.000000,0.000000,500.000000") "TraceTypeQuery1" false (Utilities|Array|MakeArray (Components|GetOwner MeshComp)) "ForDuration" true "(R=1.000000,G=0.000000,B=0.000000,A=1.000000)" "(R=0.000000,G=1.000000,B=0.000000,A=1.000000)" 2e+01))
      (Audio|PlaySoundatLocation (.Value (Utilities|Map|Find (LocalVariables|GetSound) (Variables|/Script/PhysicsCore.PhysicalMaterial|GetSurfaceType (.physmat _outhit)))) (.location _outhit) "0, 0, 0" 1.0 1.0 0.0 0 0 0 0)
      (return false))))